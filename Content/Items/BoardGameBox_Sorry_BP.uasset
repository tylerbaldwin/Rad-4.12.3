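; BoardGameBox_Sorry_BP is a board game box actor that unlocks a crystal once Rad_Blueprint has enough coins.
; On BeginPlay it hides the CrystalBP child actor and disables its collision.
; When Rad_Blueprint enters the Sphere trigger, it checks CoinCount against a 100-coin threshold, then either reveals the crystal and enables its collision or prints a shortfall message.
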(event `self.ReceiveBeginPlay`
  (`self.SetActorEnableCollision` (`ChildActorComponent.ChildActor` (`self.Crystal_BP`)) false)
  (`SceneComponent.SetVisibility` (`self.Crystal_BP`) false true))

(event `self.Sphere.OnComponentBeginOverlap`
  (params (OverlappedComponent :type "PrimitiveComponent Object Reference") (OtherActor :type "Actor Object Reference") (OtherComp :type "PrimitiveComponent Object Reference") (OtherBodyIndex :type Integer) (bFromSweep :type Boolean) (SweepResult :type "HitResult Structure (by ref)"))
  (bind _asrad_blueprint (cast `/Game/ThirdPersonBP/Blueprints/Rad_Blueprint` OtherActor))
  (if (>= (`/Game/ThirdPersonBP/Blueprints/Rad_Blueprint.Coin Count` _asrad_blueprint) 100)
    (`KismetSystemLibrary.PrintString` "You Got 100 Coins!")
    (`self.SetActorEnableCollision` (`ChildActorComponent.ChildActor` (`self.Crystal_BP`)) true)
    (`SceneComponent.SetVisibility` (`self.Crystal_BP`) true true)
    (else
      (`KismetSystemLibrary.PrintString` "Not enough coins!"))))

(fn `UserConstructionScript`)