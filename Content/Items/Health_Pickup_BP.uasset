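; Health pickup actor that restores one point of health to a Rad_Blueprint character that touches its sphere.
; The sphere overlap casts to Rad_Blueprint and acts only while Health is below the hardcoded cap of three.
; It increments Health, calls PlayerHealthHasChanged on the character, destroys itself, and spawns the Life_Explode emitter attached to the character's mesh.
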(event `self.Sphere.OnComponentBeginOverlap`
  (params (OverlappedComponent :type "PrimitiveComponent Object Reference") (OtherActor :type "Actor Object Reference") (OtherComp :type "PrimitiveComponent Object Reference") (OtherBodyIndex :type Integer) (bFromSweep :type Boolean) (SweepResult :type "HitResult Structure (by ref)"))
  (bind _asrad_blueprint (cast `/Game/ThirdPersonBP/Blueprints/Rad_Blueprint` OtherActor))
  (if (not (>= (`/Game/ThirdPersonBP/Blueprints/Rad_Blueprint.Health` _asrad_blueprint) 3))
    (set `/Game/ThirdPersonBP/Blueprints/Rad_Blueprint.Health` (+ (`/Game/ThirdPersonBP/Blueprints/Rad_Blueprint.Health` _asrad_blueprint) 1) _asrad_blueprint)
    (`/Game/ThirdPersonBP/Blueprints/Rad_Blueprint.Player Health Has Changed` _asrad_blueprint)
    (`self.K2_DestroyActor`)
    (`GameplayStatics.SpawnEmitterAttached` "/Game/ParticleSystems/Mesh/Life_Explode.Life_Explode" (`Character.Mesh` _asrad_blueprint) "None" (0.0 0.0 50.0))))

(fn `UserConstructionScript`)